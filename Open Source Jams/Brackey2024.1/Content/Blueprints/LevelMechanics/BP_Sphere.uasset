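; Physics sphere level mechanic that limits its own speed and plays impact sounds.
; Tick overrides linear velocity per axis against MaxVel and MinVel; the minimum checks are chained, correcting at most one axis per tick and only while Z is below MaxVel.
; Hit plays one of three random sounds at the impact point for the player (BP_PlayerMovement) or any component not tagged Floor.
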(event `self.ReceiveTick`
  (params (DeltaSeconds :type "Float (single-precision)"))
  (bind (_returnvalue_x _returnvalue_y _returnvalue_z) (`KismetMathLibrary.BreakVector` (`self.GetVelocity`)))
  (bind (_returnvalue_x_2 _returnvalue_y_2 _returnvalue_z_2) (`KismetMathLibrary.BreakVector` (`self.GetVelocity`)))
  (bind _sphere (`self.Sphere`))
  (bind _maxvel (`self.MaxVel`))
  (bind _sphere_2 (`self.Sphere`))
  (bind _minvel (`self.MinVel`))
  (bind _minvel_2 (`self.MinVel`))
  (if (>= _returnvalue_x_2 _maxvel)
    (`PrimitiveComponent.SetAllPhysicsLinearVelocity` _sphere_2 (`KismetMathLibrary.MakeVector` (`self.MaxVel`) _returnvalue_y_2 _returnvalue_z_2) false))
  (if (>= _returnvalue_y_2 _maxvel)
    (`PrimitiveComponent.SetAllPhysicsLinearVelocity` _sphere_2 (`KismetMathLibrary.MakeVector` _returnvalue_x_2 (`self.MaxVel`) _returnvalue_z_2) false))
  (if (>= _returnvalue_z_2 _maxvel)
    (`PrimitiveComponent.SetAllPhysicsLinearVelocity` _sphere_2 (`KismetMathLibrary.MakeVector` _returnvalue_x_2 _returnvalue_y_2 (`self.MaxVel`)) false)
    (elif (<= _returnvalue_x (`self.MinVel`))
      (`PrimitiveComponent.SetAllPhysicsLinearVelocity` _sphere (`KismetMathLibrary.MakeVector` _minvel_2 _returnvalue_y _returnvalue_z) false)
      (elif (<= _returnvalue_y _minvel)
        (`PrimitiveComponent.SetAllPhysicsLinearVelocity` _sphere (`KismetMathLibrary.MakeVector` _returnvalue_x _minvel_2 _returnvalue_z) false)
        (elif (<= _returnvalue_z _minvel)
          (`PrimitiveComponent.SetAllPhysicsLinearVelocity` _sphere (`KismetMathLibrary.MakeVector` _returnvalue_x _returnvalue_y _minvel_2) false))))))

(event `self.ReceiveHit`
  (params (MyComp :type "PrimitiveComponent Object Reference") (Other :type "Actor Object Reference") (OtherComp :type "PrimitiveComponent Object Reference") (bSelfMoved :type Boolean) (HitLocation :type "Vector Structure") (HitNormal :type "Vector Structure") (NormalImpulse :type "Vector Structure") (Hit :type "HitResult Structure (by ref)"))
  (cast `/Game/Blueprints/Player/BP_PlayerMovement` Other
    (:`then`
      (switch `int` (`KismetMathLibrary.RandomIntegerInRange` 1 3) :!label _label
        (:`1`
          (`GameplayStatics.PlaySoundAtLocation` "/Game/Audio/SphereHitSound1.SphereHitSound1" HitLocation (struct) 1.0 1.0 0.0 "/Game/Audio/BigSFXAttenuation.BigSFXAttenuation" "/Game/Audio/BallHitConcurrency.BallHitConcurrency" null null))
        (:`2`
          (`GameplayStatics.PlaySoundAtLocation` "/Game/Audio/SphereHitSound2.SphereHitSound2" HitLocation (struct) 1.0 1.0 0.0 "/Game/Audio/BigSFXAttenuation.BigSFXAttenuation" "/Game/Audio/BallHitConcurrency.BallHitConcurrency" null null))
        (:`3`
          (`GameplayStatics.PlaySoundAtLocation` "/Game/Audio/SphereHitSound3.SphereHitSound3" HitLocation (struct) 1.0 1.0 0.0 "/Game/Audio/BigSFXAttenuation.BigSFXAttenuation" "/Game/Audio/BallHitConcurrency.BallHitConcurrency" null null))))
    (:`CastFailed`
      (if (not (`ActorComponent.ComponentHasTag` OtherComp "Floor"))
        (goto _label)))))

(fn `UserConstructionScript`)