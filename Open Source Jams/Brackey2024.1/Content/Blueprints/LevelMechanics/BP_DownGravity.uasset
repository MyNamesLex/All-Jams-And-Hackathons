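; BP_DownGravity is a level-mechanic volume that applies vertical force, DownForcePlayer, to the player and components inside its Cube.
; Cube overlaps track the player and an array of other components, zeroing entering components' velocity if the Cube itself has gravity enabled.
; A delay-gated Tick pushes both through AddForce, using the same force value.
; Two looping Delay chains scroll arrow indicators downward, resetting them at the bottom.
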(event `LoopMoveArrowDown2`
  (bind _downarrow1 (`self.DownArrow1`))
  (bind (_relativelocation_x _relativelocation_y _relativelocation_z) (`KismetMathLibrary.BreakVector` (`SceneComponent.RelativeLocation` (`self.DownArrow1`))))
  (bind (_relativelocation_x_2 _relativelocation_y_2 _relativelocation_z_2) (`KismetMathLibrary.BreakVector` (`SceneComponent.RelativeLocation` _downarrow1)))
  (`SceneComponent.K2_SetRelativeLocation` _downarrow1 (`KismetMathLibrary.MakeVector` 0.0 -10.0 (- _relativelocation_z_2 0.5)) false false :!label _label)
  (`KismetSystemLibrary.Delay` 0.1)
  (if (<= _relativelocation_z -42.2)
    (`SceneComponent.K2_SetRelativeLocation` (`self.DownArrow1`) (0.0 -10.0 38.0) false false)
    (`KismetSystemLibrary.Delay` 0.1)
    (goto _label)
    (else
      (goto _label))))

(event `self.ReceiveBeginPlay`
  (`self.LoopMoveArrowDown`)
  (`self.LoopMoveArrowDown2`))

(event `LoopMoveArrowDown`
  (bind _downarrow (`self.DownArrow`))
  (bind (_relativelocation_x _relativelocation_y _relativelocation_z) (`KismetMathLibrary.BreakVector` (`SceneComponent.RelativeLocation` _downarrow)))
  (bind (_relativelocation_x_2 _relativelocation_y_2 _relativelocation_z_2) (`KismetMathLibrary.BreakVector` (`SceneComponent.RelativeLocation` (`self.DownArrow`))))
  (`SceneComponent.K2_SetRelativeLocation` _downarrow (`KismetMathLibrary.MakeVector` 0.0 -10.0 (- _relativelocation_z 0.5)) false false :!label _label_2)
  (`KismetSystemLibrary.Delay` 0.1)
  (if (<= _relativelocation_z_2 -42.2)
    (`SceneComponent.K2_SetRelativeLocation` (`self.DownArrow`) (0.0 -10.0 38.0) false false)
    (`KismetSystemLibrary.Delay` 0.1)
    (goto _label_2)
    (else
      (goto _label_2))))

(event `self.ReceiveTick`
  (params (DeltaSeconds :type "Float (single-precision)"))
  (`KismetSystemLibrary.Delay` (`self.FloatForceDelay`))
  (if (`self.PlayerCollided`)
    (`self.FloatUpPlayer` (`self.Player`)))
  (if (`self.CompCollided`)
    (for _array_element (`self.Components`)
      (`self.FloatCompUp` _array_element))))

(event `self.Cube.OnComponentBeginOverlap`
  (params (OverlappedComponent :type "PrimitiveComponent Object Reference") (OtherActor :type "Actor Object Reference") (OtherComp :type "PrimitiveComponent Object Reference") (OtherBodyIndex :type Integer) (bFromSweep :type Boolean) (SweepResult :type "HitResult Structure (by ref)"))
  (bind _asbp_player_movement (cast `/Game/Blueprints/Player/BP_PlayerMovement` OtherActor)
    (:`then`
      (set `self.Player` _asbp_player_movement)
      (set `self.PlayerCollided` true))
    (:`CastFailed`
      (if (`PrimitiveComponent.IsGravityEnabled` OverlappedComponent)
        (`PrimitiveComponent.SetAllPhysicsLinearVelocity` OtherComp (0.0 0.0 0.0) false)
        (`KismetArrayLibrary.Array_Add` (`self.Components`) OtherComp)
        (set `self.CompCollided` true)))))

(event `self.Cube.OnComponentEndOverlap`
  (params (OverlappedComponent :type "PrimitiveComponent Object Reference") (OtherActor :type "Actor Object Reference") (OtherComp :type "PrimitiveComponent Object Reference") (OtherBodyIndex :type Integer))
  (bind _components (`self.Components`))
  (cast `/Game/Blueprints/Player/BP_PlayerMovement` OtherActor
    (:`then`
      (set `self.PlayerCollided` false))
    (:`CastFailed`
      (if (`KismetArrayLibrary.Array_Contains` (`self.Components`) OtherComp)
        (`KismetArrayLibrary.Array_RemoveItem` _components OtherComp)
        (if (`KismetArrayLibrary.Array_IsEmpty` _components)
          (set `self.CompCollided` false))))))

(event `FloatUpPlayer`
  (params (Player :type "/Game/Blueprints/Player/BP_PlayerMovement Object Reference"))
  (`CharacterMovementComponent.AddForce` (`Character.CharacterMovement` Player) (`KismetMathLibrary.MakeVector` 0.0 0.0 (`self.DownForcePlayer`))))

(event `FloatCompUp`
  (params (Component :type "PrimitiveComponent Object Reference"))
  (`PrimitiveComponent.AddForce` Component (`KismetMathLibrary.MakeVector` 0.0 0.0 (`self.DownForcePlayer`)) "None" false))

(fn `UserConstructionScript`)