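; BP_DroppableWall is a level-mechanic wall that can break with sound and stone particle effects.
; Its WallBreakVFX event always plays the break sound at the actor's location.
; When its Destroy flag is set, it also activates five stone effects, hides the wall mesh, disables its collision and destroys the actor after a short delay.
; The file contains no drop logic or internal trigger for the event.
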(event `self.WallBreakVFX`
  (params (Destroy :type Boolean))
  (bind _wall (`self.Wall`))
  (`GameplayStatics.PlaySoundAtLocation` "/Game/Audio/WallBreakSFX.WallBreakSFX" (`self.K2_GetActorLocation`) (struct) 1.0 1.0 0.0 null null null null)
  (if Destroy
    (`ActorComponent.Activate` (`self.P_WallBreak_Stone`) false)
    (`ActorComponent.Activate` (`self.P_WallBreak_Stone1`) false)
    (`ActorComponent.Activate` (`self.P_WallBreak_Stone2`) false)
    (`ActorComponent.Activate` (`self.P_WallBreak_Stone3`) false)
    (`ActorComponent.Activate` (`self.P_WallBreak_Stone4`) false)
    (`SceneComponent.SetVisibility` _wall false false)
    (`PrimitiveComponent.SetCollisionEnabled` _wall "NoCollision")
    (`KismetSystemLibrary.Delay` 4.0)
    (`self.K2_DestroyActor`)))

(fn `UserConstructionScript`)