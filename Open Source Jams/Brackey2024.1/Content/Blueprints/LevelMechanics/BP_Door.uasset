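; BP_Door is a level exit door that opens with an animation and sound and loads the next level.
; PlayOpenDoorAnim plays the door animation and SFX, then stops the animation after a fixed delay.
; Overlapping NextLevelTrigger with BP_PlayerMovement adds its local time to BP_GameInstance's total, then opens NextLevelName after a short delay.
; A failed player cast prints an error and retries the same actor in a delayed loop.
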(event `self.PlayOpenDoorAnim`
  (bind _door (`self.Door`))
  (`SkeletalMeshComponent.PlayAnimation` _door "/Game/Assets/door-wood/source/OpenDoor.OpenDoor" false)
  (`GameplayStatics.PlaySoundAtLocation` "/Game/Audio/Door_Open_SFX.Door_Open_SFX" (`self.K2_GetActorLocation`) (struct) 1.0 1.0 0.0 "/Game/Audio/BigSFXAttenuation.BigSFXAttenuation" null null null)
  (`KismetSystemLibrary.Delay` 1.1)
  (`SkeletalMeshComponent.Stop` _door))

(event `self.NextLevelTrigger.OnComponentBeginOverlap`
  (params (OverlappedComponent :type "PrimitiveComponent Object Reference") (OtherActor :type "Actor Object Reference") (OtherComp :type "PrimitiveComponent Object Reference") (OtherBodyIndex :type Integer) (bFromSweep :type Boolean) (SweepResult :type "HitResult Structure (by ref)"))
  (bind _asbp_player_movement (cast `/Game/Blueprints/Player/BP_PlayerMovement` OtherActor :!label _label)
    (:`then`
      (bind _asbp_game_instance (cast `/Game/Blueprints/GameModes/BP_GameInstance` (`GameplayStatics.GetGameInstance`)))
      (set `/Game/Blueprints/GameModes/BP_GameInstance.Time` (+ (`/Game/Blueprints/GameModes/BP_GameInstance.Time` _asbp_game_instance) (`PlayerMovement.TimeLocal` _asbp_player_movement)) _asbp_game_instance)
      (`KismetSystemLibrary.Delay` 0.2)
      (`GameplayStatics.OpenLevel` (`self.NextLevelName`)))
    (:`CastFailed`
      (`KismetSystemLibrary.Delay` 0.2)
      (`KismetSystemLibrary.PrintString` "CAST FAILED BP PLAYERMOVMENT BP DOOR")
      (goto _label))))

(fn `UserConstructionScript`)