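; Anti-gravity volume that pushes the player and other components upward while they overlap its Cube trigger.
; Overlap events track the player and a component list, adding non-player components only if the Cube itself has gravity enabled.
; A delayed Tick applies upward force, zeroing player velocity on first contact and lifting components only when no player is inside.
; Two looping events animate rising arrow indicators.
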(event `self.ReceiveTick`
  (params (DeltaSeconds :type "Float (single-precision)"))
  (`KismetSystemLibrary.Delay` (`self.FloatForceDelay`))
  (if (`self.PlayerCollided`)
    (`self.FloatUpPlayer` (`self.Player`))
    (if (not (`self.PlayerFirstCollide`))
      (set `self.PlayerFirstCollide` true)
      (set `MovementComponent.Velocity` (0.0 0.0 0.0) (`Character.CharacterMovement` (`self.Player`))))
    (elif (`self.CompCollided`)
      (for _array_element (`self.Components`)
        (`self.FloatCompUp` _array_element)))))

(event `self.ReceiveBeginPlay`
  (`self.LoopMoveArrowUp`)
  (`self.LoopMoveArrowUp2`))

(event `self.Cube.OnComponentBeginOverlap`
  (params (OverlappedComponent :type "PrimitiveComponent Object Reference") (OtherActor :type "Actor Object Reference") (OtherComp :type "PrimitiveComponent Object Reference") (OtherBodyIndex :type Integer) (bFromSweep :type Boolean) (SweepResult :type "HitResult Structure (by ref)"))
  (bind _asbp_player_movement (cast `/Game/Blueprints/Player/BP_PlayerMovement` OtherActor)
    (:`then`
      (set `self.Player` _asbp_player_movement)
      (set `self.PlayerCollided` true))
    (:`CastFailed`
      (if (`PrimitiveComponent.IsGravityEnabled` OverlappedComponent)
        (`KismetArrayLibrary.Array_Add` (`self.Components`) OtherComp)
        (set `self.CompCollided` true)))))

(event `self.Cube.OnComponentEndOverlap`
  (params (OverlappedComponent :type "PrimitiveComponent Object Reference") (OtherActor :type "Actor Object Reference") (OtherComp :type "PrimitiveComponent Object Reference") (OtherBodyIndex :type Integer))
  (bind _components (`self.Components`))
  (cast `/Game/Blueprints/Player/BP_PlayerMovement` OtherActor
    (:`then`
      (set `self.PlayerCollided` false)
      (set `self.PlayerFirstCollide` false))
    (:`CastFailed`
      (if (`KismetArrayLibrary.Array_Contains` (`self.Components`) OtherComp)
        (`KismetArrayLibrary.Array_RemoveItem` _components OtherComp)
        (if (`KismetArrayLibrary.Array_IsEmpty` _components)
          (set `self.CompCollided` false))))))

(event `FloatUpPlayer`
  (params (Player :type "/Game/Blueprints/Player/BP_PlayerMovement Object Reference"))
  (if (not (== Player null))
    (`CharacterMovementComponent.AddForce` (`Character.CharacterMovement` Player) (`KismetMathLibrary.MakeVector` 0.0 0.0 (`self.UpForcePlayer`)))))

(event `FloatCompUp`
  (params (Component :type "PrimitiveComponent Object Reference"))
  (`PrimitiveComponent.AddForce` Component (`KismetMathLibrary.MakeVector` 0.0 0.0 (`self.UpForcePlayer`)) "None" false))

(event `LoopMoveArrowUp2`
  (bind _3d_rightarrow_arrow2 (`self.3D_RightArrow_Arrow2`))
  (bind (_relativelocation_x _relativelocation_y _relativelocation_z) (`KismetMathLibrary.BreakVector` (`SceneComponent.RelativeLocation` _3d_rightarrow_arrow2)))
  (bind (_relativelocation_x_2 _relativelocation_y_2 _relativelocation_z_2) (`KismetMathLibrary.BreakVector` (`SceneComponent.RelativeLocation` (`self.3D_RightArrow_Arrow2`))))
  (`SceneComponent.K2_SetRelativeLocation` _3d_rightarrow_arrow2 (`KismetMathLibrary.MakeVector` 0.0 0.0 (+ _relativelocation_z 0.5)) false false :!label _label)
  (`KismetSystemLibrary.Delay` 0.1)
  (if (>= _relativelocation_z_2 34.2)
    (`SceneComponent.K2_SetRelativeLocation` (`self.3D_RightArrow_Arrow2`) (0.0 0.0 -45.400002) false false)
    (`KismetSystemLibrary.Delay` 0.1)
    (goto _label)
    (else
      (goto _label))))

(event `LoopMoveArrowUp`
  (bind _3d_rightarrow_arrow1 (`self.3D_RightArrow_Arrow1`))
  (bind (_relativelocation_x _relativelocation_y _relativelocation_z) (`KismetMathLibrary.BreakVector` (`SceneComponent.RelativeLocation` (`self.3D_RightArrow_Arrow1`))))
  (bind (_relativelocation_x_2 _relativelocation_y_2 _relativelocation_z_2) (`KismetMathLibrary.BreakVector` (`SceneComponent.RelativeLocation` _3d_rightarrow_arrow1)))
  (`SceneComponent.K2_SetRelativeLocation` _3d_rightarrow_arrow1 (`KismetMathLibrary.MakeVector` 0.0 0.0 (+ _relativelocation_z_2 0.5)) false false :!label _label_2)
  (`KismetSystemLibrary.Delay` 0.1)
  (if (>= _relativelocation_z 34.2)
    (`SceneComponent.K2_SetRelativeLocation` (`self.3D_RightArrow_Arrow1`) (0.0 0.0 -45.400002) false false)
    (`KismetSystemLibrary.Delay` 0.1)
    (goto _label_2)
    (else
      (goto _label_2))))

(fn `UserConstructionScript`)