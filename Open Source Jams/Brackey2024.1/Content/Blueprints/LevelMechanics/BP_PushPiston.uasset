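; BP_PushPiston is a level-mechanic piston that launches whatever enters its TriggerSide volume along its Arrow's forward vector.
; Each overlap plays a spring sound at the actor, then applies an impulse scaled by PistonForce.
; BP_PlayerMovement characters get a quarter-strength impulse through CharacterMovement, with ground friction zeroed and restored to a fixed value after a delay.
; Anything else receives the full impulse on the overlapping component.
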(event `self.TriggerSide.OnComponentBeginOverlap`
  (params (OverlappedComponent :type "PrimitiveComponent Object Reference") (OtherActor :type "Actor Object Reference") (OtherComp :type "PrimitiveComponent Object Reference") (OtherBodyIndex :type Integer) (bFromSweep :type Boolean) (SweepResult :type "HitResult Structure (by ref)"))
  (`GameplayStatics.PlaySoundAtLocation` "/Game/Audio/SpringSFX.SpringSFX" (`self.K2_GetActorLocation`) (struct) 1.0 1.0 0.0 "/Game/Audio/VBigSFXAttenuation.VBigSFXAttenuation" null null null)
  (bind _asbp_player_movement (cast `/Game/Blueprints/Player/BP_PlayerMovement` OtherActor)
    (:`then`
      (bind _charactermovement (`Character.CharacterMovement` _asbp_player_movement))
      (set `CharacterMovementComponent.GroundFriction` 0.0 _charactermovement)
      (`CharacterMovementComponent.AddImpulse` _charactermovement (* (`SceneComponent.GetForwardVector` (`self.Arrow`)) (/ (`self.PistonForce`) 4.0)) false)
      (`KismetSystemLibrary.Delay` 3.0)
      (set `CharacterMovementComponent.GroundFriction` 8.0 (`Character.CharacterMovement` _asbp_player_movement)))
    (:`CastFailed`
      (`PrimitiveComponent.AddImpulse` OtherComp (* (`SceneComponent.GetForwardVector` (`self.Arrow`)) (`self.PistonForce`)) "None" false))))

(fn `UserConstructionScript`)