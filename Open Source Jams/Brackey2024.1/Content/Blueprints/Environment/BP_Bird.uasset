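; BP_Bird is an environment bird that gets scared off once, when something first overlaps its ScareRadius and triggers FlyAway.
; Custom events play idle, takeoff and flight animations, with takeoff chaining on a delay and a polling loop leading into looping flight.
; Despite its name, FlytoRandomReachableLocation sends the bird to MoveToObj's location, applying a look-at rotation with a yaw offset.
; An unused random navmesh destination picker remains, noted as broken.
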(event `self.ReceiveBeginPlay`)

(event `self.PlayIdleAnim`
  (`SkeletalMeshComponent.PlayAnimation` (`self.Bird`) "/Game/Assets/Bird/source/bird_animations__2__Anim_idleA1_bird.bird_animations__2__Anim_idleA1_bird" true))

(event `self.FlyToRandomReachableLocation`
  (bind _movetoobj (`self.MoveToObj`))
  (bind (_returnvalue_roll _returnvalue_pitch _returnvalue_yaw) (`KismetMathLibrary.BreakRotator` (`KismetMathLibrary.FindRelativeLookAtRotation` (`self.GetTransform` _movetoobj) (`self.K2_GetActorLocation`))))
  (set `self.RandomReachableLocationFVector` (`self.K2_GetActorLocation` _movetoobj))
  (`SceneComponent.K2_SetRelativeRotation` (`self.Bird`) (`KismetMathLibrary.MakeRotator` _returnvalue_roll _returnvalue_pitch (+ _returnvalue_yaw 90.0)) false true)
  (`self.MoveToLocation` (`self.RandomReachableLocationFVector`)))

(event `self.ScareRadius.OnComponentBeginOverlap`
  (params (OverlappedComponent :type "PrimitiveComponent Object Reference") (OtherActor :type "Actor Object Reference") (OtherComp :type "PrimitiveComponent Object Reference") (OtherBodyIndex :type Integer) (bFromSweep :type Boolean) (SweepResult :type "HitResult Structure (by ref)"))
  (if (not (`self.AlreadyScared`))
    (set `self.AlreadyScared` true)
    (`self.FlyAway`)))

(event `self.PlayTakeoffAnim`
  (`SkeletalMeshComponent.PlayAnimation` (`self.Bird`) "/Game/Assets/Bird/source/bird_animations__2__Anim_fly_startA_bird.bird_animations__2__Anim_fly_startA_bird" false)
  (`KismetSystemLibrary.Delay` (`self.TimeUntilNormalFly`))
  (`self.PlayNormalFlyAnim`))

(event `self.PlayNormalFlyAnim`
  (bind _bird (`self.Bird`))
  (`SkeletalMeshComponent.PlayAnimation` _bird "/Game/Assets/Bird/source/bird_animations__2__Anim_fly1_bird.bird_animations__2__Anim_fly1_bird" false)
  (if (`SkeletalMeshComponent.IsPlaying` _bird) :!label _label
    (`KismetSystemLibrary.Delay` 0.2)
    (goto _label)
    (else
      (`SkeletalMeshComponent.PlayAnimation` (`self.Bird`) "/Game/Assets/Bird/source/bird_animations__2__Anim_fly3_bird.bird_animations__2__Anim_fly3_bird" true))))

(fn `UserConstructionScript`)