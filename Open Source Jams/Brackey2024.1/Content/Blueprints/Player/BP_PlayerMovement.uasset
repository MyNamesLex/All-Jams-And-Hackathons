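; Player character Blueprint that manages HUD, pause menu, gravity-zone feedback and the enabling or locking of movement and camera.
; It creates the player UI on BeginPlay and exposes events for tip prompts and a reset-button click sound.
; Pause menu events show or remove the menu, toggling the cursor and player control through TogglePlayerActive.
; Overlapping up or down gravity volumes adds a tint widget, which is removed on exit.
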(event `TogglePlayerActive`
  (params (PlayerActive :type Boolean))
  (bind _camera (`self.Camera`))
  (if PlayerActive
    (set `CameraComponent.bUsePawnControlRotation` true _camera)
    (set `self.WalkSpeed` 600.0)
    (set `self.LockPlayerCamera` false)
    (else
      (set `CameraComponent.bUsePawnControlRotation` false _camera)
      (set `self.WalkSpeed` 0.0)
      (set `self.LockPlayerCamera` true))))

(event `self.ReceiveBeginPlay`
  (bind _returnvalue (`|CreateWidget` "/Game/Blueprints/UI/BP_PlayerUI.BP_PlayerUI_C" (`GameplayStatics.GetPlayerController` 0)))
  (bind _output_get (set `self.Player Ui` _returnvalue))
  (`UserWidget.AddToViewport` _output_get 0))

(event `self.ReceiveActorBeginOverlap`
  (params (OtherActor :type "Actor Object Reference"))
  (cast `/Game/Blueprints/LevelMechanics/BP_UpGravity` OtherActor
    (:`then`
      _)
    (:`CastFailed`
      (cast `/Game/Blueprints/LevelMechanics/BP_DownGravity` OtherActor)))
  (if (not (!= (`self.PlayerGravityTint`) null))
    (bind _returnvalue (`|CreateWidget` "/Game/Blueprints/UI/BP_PlayerGravityTint.BP_PlayerGravityTint_C"))
    (bind _output_get (set `self.PlayerGravityTint` _returnvalue))
    (`UserWidget.AddToViewport` _output_get 0)))

(event `self.HidePauseMenu`
  (`Widget.RemoveFromParent` (`self.Player Pause Menu`))
  (`GameplayStatics.SetGamePaused` false)
  (set `PlayerController.bShowMouseCursor` false (`GameplayStatics.GetPlayerController` 0))
  (`self.TogglePlayerActive` true))

(event `self.ShowPauseMenu`
  (bind _returnvalue (`|CreateWidget` "/Game/Blueprints/UI/BP_PlayerPauseMenu.BP_PlayerPauseMenu_C" (`GameplayStatics.GetPlayerController` 0)))
  (bind _output_get (set `self.Player Pause Menu` _returnvalue))
  (`UserWidget.AddToViewport` _output_get 0)
  (`self.TogglePlayerActive` false)
  (set `PlayerController.bShowMouseCursor` true (`GameplayStatics.GetPlayerController` 0)))

(event `self.ReceiveTick`
  (params (DeltaSeconds :type "Float (single-precision)")))

(event `self.ReceiveActorEndOverlap`
  (params (OtherActor :type "Actor Object Reference"))
  (cast `/Game/Blueprints/LevelMechanics/BP_UpGravity` OtherActor
    (:`then`
      _)
    (:`CastFailed`
      (cast `/Game/Blueprints/LevelMechanics/BP_DownGravity` OtherActor)))
  (`Widget.RemoveFromParent` (`self.PlayerGravityTint`))
  (set `self.PlayerGravityTint` null))

(event `self.ShowTip`
  (`/Game/Blueprints/UI/BP_PlayerUI.TipSwitch` (`self.Player Ui`))
  (set `self.isShowingTip` true))

(event `self.ShowTipKey`
  (bind _player_ui (`self.Player Ui`))
  (bind _showtiptext (`/Game/Blueprints/UI/BP_PlayerUI.ShowTipText` _player_ui))
  (`Widget.SetVisibility` _showtiptext "Visible")
  (`TextBlock.SetText` _showtiptext "Show Tip")
  (`Widget.SetVisibility` (`/Game/Blueprints/UI/BP_PlayerUI.KeySprite` _player_ui) "Visible"))

(event `self.HideTipKey`
  (bind _player_ui (`self.Player Ui`))
  (`TextBlock.SetText` (`/Game/Blueprints/UI/BP_PlayerUI.ShowTipText` _player_ui) "Hide Tip")
  (`Widget.SetVisibility` (`/Game/Blueprints/UI/BP_PlayerUI.KeySprite` _player_ui) "Visible"))

(event `self.HideTip`
  (`Widget.SetVisibility` (`/Game/Blueprints/UI/BP_PlayerUI.TipText` (`self.Player Ui`)) "Hidden")
  (set `self.isShowingTip` false))

(event `self.PlayResetButtonSFX`
  (params (ButtonLocation :type "Vector Structure"))
  (`GameplayStatics.PlaySoundAtLocation` "/Game/Audio/Click.Click" ButtonLocation (struct) 1.0 1.0 0.0 "/Game/Audio/VBigSFXAttenuation.VBigSFXAttenuation" null null null))

(fn `UserConstructionScript`)